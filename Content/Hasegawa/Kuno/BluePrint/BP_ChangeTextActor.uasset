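; BP_ChangeTextActor is an actor that shows two text sprites in sequence in response to clicks.
; Show01 starts transparent, and EV_click plays the Change timeline to crossfade alpha from Show02 to Show01.
; When the timeline finishes it advances the click counter, so the next click calls CallEVChangeLevel to request a level change.
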(event `self.ReceiveBeginPlay`
  (`PaperSpriteComponent.SetSpriteColor` (`self.show01`) (make `LinearColor` 1.0 1.0 1.0 0.0)))

(event `EV_click`
  (if (== (`self.cnt_clickSeqence`) 1)
    (`self.EV_changeLevel`)
    (else
      (bind (_direction `_新規track_0`) (`Timeline|change`)
        (:`Update`
          (`PaperSpriteComponent.SetSpriteColor` (`self.show01`) (make `LinearColor` 1.0 1.0 1.0 `_新規track_0`))
          (`PaperSpriteComponent.SetSpriteColor` (`self.show02`) (make `LinearColor` 1.0 1.0 1.0 (- 1.0 `_新規track_0`))))
        (:`Finished`
          (set `self.cnt_clickSeqence` 1))))))

(fn `FC_init`)

(fn `UserConstructionScript`)