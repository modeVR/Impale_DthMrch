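; BP_DragAndDropPlayer is a player Blueprint that grabs and releases clickable objects with the left mouse button.
; An IsHitclickable macro gates press and release on HitClickable, which, like HitObject, is not set in this graph.
; Press calls OnClick on HitObject and attaches it to the SpringArm through a cast; release calls LeaveClick and DetachThis.
; Unconnected attach and detach component nodes remain unused.
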(event `Key|LeftMouseButton`
  (params (Key :type "Key Structure" :default "AnyKey"))
  (bind _hitobject (`self.HitObject`))
  (bind _asbbp_drag_and_drop_object (cast `` _hitobject :!pure true))
  (:`Pressed`
    (`self.IsHitclickable`
      (:`true`
        (`self.OnClick` _hitobject)
        (`self.AttachThis` _asbbp_drag_and_drop_object (`self.SpringArm`)))))
  (:`Released`
    (`self.IsHitclickable`
      (:`true`
        (`self.LeaveClick` _hitobject)
        (`self.DetachThis` _asbbp_drag_and_drop_object)))))

(fn `UserConstructionScript`
  (`parent.UserConstructionScript`))