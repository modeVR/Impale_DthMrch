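; Blueprint function library with shared helpers for stage selection and screen fades.
; SelectLevel converts the chosen stage to an integer, looks up the matching entry in a level name array and opens that level by name.
; FadeAction plays the FadeOut or FadeIn animation on the widget passed to it, with a Fade value of zero choosing FadeOut.
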(fn `FadeAction`
  (params (NewParam :type "Object Object Reference") (Fade :type Byte))
  (if (== Fade 0)
    (`UserWidget.PlayAnimation` NewParam (`/Game/Hasegawa/hasegawa/Blueprints/BP_FunctionLib.FadeOut` NewParam) 0.0 1 "Forward" 1.0)
    (else
      (`UserWidget.PlayAnimation` NewParam (`/Game/Hasegawa/hasegawa/Blueprints/BP_FunctionLib.FadeIn` NewParam) 0.0 1 "Forward" 1.0))))

(fn `SelectLevel`
  (params (SelectStarge :type Byte))
  (locals (LevelName :type "Array of Name"))
  (`GameplayStatics.OpenLevel` null (`KismetArrayLibrary.Array_Get` (`local.LevelName`) (`KismetMathLibrary.Conv_ByteToInt` SelectStarge))))