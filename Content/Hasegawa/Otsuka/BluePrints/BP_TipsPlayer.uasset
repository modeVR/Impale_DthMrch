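; BP_TipsPlayer is a player Blueprint, apparently for a tips scene, that lets the player look around and move on with a click.
; Yaw input adds world rotation to the Camera and pitch input adds local rotation, which keeps the two axes from introducing roll.
; Pressing Click calls EVOpenLevelMain, which by its name signals opening the main level.
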(event `InputAxis|CameraRotationYaw`
  (params (AxisValue :type "Float (single-precision)"))
  (`SceneComponent.K2_AddWorldRotation` (`self.Camera`) (`KismetMathLibrary.MakeRotator` 0.0 0.0 AxisValue) false false))

(event `InputAxis|CameraRotationPitch`
  (params (AxisValue :type "Float (single-precision)"))
  (`SceneComponent.K2_AddLocalRotation` (`self.Camera`) (`KismetMathLibrary.MakeRotator` 0.0 AxisValue) false false))

(event `InputAction|Click`
  (params (Key :type "Key Structure" :default "AnyKey"))
  (:`Pressed`
    (`self.EV_OpenLevelMain`)))

(fn `UserConstructionScript`
  (`parent.UserConstructionScript`))