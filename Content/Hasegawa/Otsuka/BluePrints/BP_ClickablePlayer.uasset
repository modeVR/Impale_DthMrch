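; VR player that enables the HMD on start, rotates its camera from input axes and clicks objects by gaze.
; A per-tick camera line trace tracks the clickable object under view, passing it the impact point and click and leave calls from the Click input.
; Any capsule overlap or the A debug key plays a death sound and calls the player-death dispatch.
; A timeline drives an X-axis shake, and P takes a high-resolution screenshot.
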(event `InputAxis|CameraRotationYaw`
  (params (AxisValue :type "Float (single-precision)"))
  (`SceneComponent.K2_AddWorldRotation` (`self.Camera`) (`KismetMathLibrary.MakeRotator` 0.0 0.0 AxisValue) false false))

(event `Key|P`
  (params (Key :type "Key Structure" :default "AnyKey"))
  (:`Pressed`
    (`KismetSystemLibrary.ExecuteConsoleCommand` "HighResShot 4677x6622")))

(event `InputAxis|CameraRotationPitch`
  (params (AxisValue :type "Float (single-precision)"))
  (`SceneComponent.K2_AddLocalRotation` (`self.Camera`) (`KismetMathLibrary.MakeRotator` 0.0 AxisValue) false false))

(event `HMDActivation`
  ;[1 1 1] HMDをアクティベーションするイベント
  (`HeadMountedDisplayFunctionLibrary.EnableHMD` true)
  (if (`HeadMountedDisplayFunctionLibrary.IsHeadMountedDisplayEnabled`)
    (`KismetSystemLibrary.ExecuteConsoleCommand` "stereo on")))

(event `self.ReceiveBeginPlay`
  (`self.HMDActivation`))

(event `self.ReceiveTick`
  (params (DeltaSeconds :type "Float (single-precision)"))
  (bind _returnvalue (`SceneComponent.K2_GetComponentLocation` (`self.Camera`)))
  ;[1 1 1] ライントレースの発動
  (bind _outhit (`KismetSystemLibrary.LineTraceSingle` :`Start` _returnvalue :`End` (+ _returnvalue (* (`SceneComponent.GetForwardVector` (`self.Camera`)) (`self.LookDistance`))) :`TraceChannel` "TraceTypeQuery1" :`DrawDebugType` "ForOneFrame"))
  (bind (_bblockinghit _binitialoverlap _time _location _impactpoint _normal _impactnormal _physmat _hitactor) (`GameplayStatics.BreakHitResult` _outhit))
  ;[1 1 1] 視線の先のオブジェクトがClick可能オブジェクトか？
  (set `self.t_impactPoint` _impactpoint)
  (cast `` _hitactor
    (:`then`
      (set `self.t_hitObject` null)
      (`self.IsClickableObject`))
    (:`CastFailed`
      (`self.IsNotClickableObject`))))

(event `IsClickableObject`
  ;[1 1 1] 視線の先のオブジェクトがClick可能オブジェクトか？
  (`/Engine/EditorBlueprintResources/StandardMacros.IsValid` null
    (:`Is Valid`
      (if (not (== null null))
        (`self.LeaveClick` null)
        (set `self.HitObject` null :!label _label)))
    (:`Is Not Valid`
      (goto _label)))
  (`self.ReciveEyeTrack` (`self.t_impactPoint`))
  (`self.ClickJudge`)
  (set `self.hitClickable` true))

(event `InputAction|Click`
  (params (Key :type "Key Structure" :default "AnyKey"))
  ;[1 1 1] クリックボタンを操作時の動作
  (:`Pressed`
    (`self.IsHitClickable`
      (:`true`
        (`self.OnClick`))))
  (:`Released`
    (`self.IsHitClickable`
      (:`true`
        (`self.LeaveClick`)))))

(event `ClickJudge`
  ;[1 1 1] クリックボタンを操作時の動作
)

(event `Key|A`
  (params (Key :type "Key Structure" :default "AnyKey"))
  (:`Pressed`
    (`KismetSystemLibrary.PrintString` "Hello" :!label _label_2)
    (`self.PlaySound` (`self.dead`) (0.0 0.0 0.0))
    (`self.DeadPlayer`)))

(event `IsNotClickableObject`
  ;[1 1 1] clickableObjectではなかった時の処理
  (`/Engine/EditorBlueprintResources/StandardMacros.IsValid` null
    (:`Is Valid`
      (`self.LeaveClick` null)
      (set `self.hitClickable` false)
      (set `self.HitObject` null))))

(event `self.CapsuleComponent.OnComponentBeginOverlap`
  (params (OverlappedComponent :type "PrimitiveComponent Object Reference") (OtherActor :type "Actor Object Reference") (OtherComp :type "PrimitiveComponent Object Reference") (OtherBodyIndex :type Integer) (bFromSweep :type Boolean) (SweepResult :type "HitResult Structure (by ref)"))
  (goto _label_2))

(event `EV_Shake`
  (params (ShakeTime :type "Float (double-precision)") (SwingWidth :type "Float (double-precision)"))
  (bind (_returnvalue_x _returnvalue_y _returnvalue_z) (`KismetMathLibrary.BreakVector` (`self.K2_GetActorLocation`)))
  (bind _pos_evshakebaf_x (`KismetMathLibrary.BreakVector` (`self.pos_EVShakeBaf`)))
  ;[1 1 1] シェイク
  (if (not (`self.flg_EVShakeNow`))
    (set `self.flg_EVShakeNow` true)
    (set `self.pos_EVShakeBaf` (`self.K2_GetActorLocation`))
    (`TimelineComponent.SetPlayRate` (`self.Shake TimeLine`) (/ 1.0 ShakeTime))
    (bind (_direction `_新規track_0`) (`Timeline|Shake TimeLine` :!via `PlayFromStart`)
      (:`Update`
        (`self.K2_SetActorLocation` (`KismetMathLibrary.MakeVector` (+ (* SwingWidth `_新規track_0`) _pos_evshakebaf_x) _returnvalue_y _returnvalue_z)))
      (:`Finished`
        (set `self.flg_EVShakeNow` false)))))

(fn `UserConstructionScript`)